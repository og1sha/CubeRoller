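; BP_Cloud is a cloud actor that drifts back and forth endlessly between a start point and an end point.
; On BeginPlay it snaps the Cloud component to StartLocation, then two timelines alternate, each lerping the world position to the opposite point and triggering the other when finished.
; At the start of each leg, RandomizeScale gives the cloud a new random, non-uniform scale to vary its shape.
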(event Custom|MoveFromStartLocation
  (CallFunction|RandomizeScale)
  (bind _alpha (Timeline|Timeline_0 PlayFromStart)
    (:Update
      (Transformation|SetWorldLocation (Variables|Default|GetCloud) (Math|Vector|Lerp(Vector) (Transformation|GetWorldLocation (Variables|Default|GetStartLocation)) (Transformation|GetWorldLocation (Variables|Default|GetEndLocation)) _alpha) false false))
    (:Finished
      (CallFunction|MovefromEndLocation))))

(event Custom|MoveFromEndLocation
  (CallFunction|RandomizeScale)
  (bind _alpha (Timeline|Timeline_1 PlayFromStart)
    (:Update
      (Transformation|SetWorldLocation (Variables|Default|GetCloud) (Math|Vector|Lerp(Vector) (Transformation|GetWorldLocation (Variables|Default|GetEndLocation)) (Transformation|GetWorldLocation (Variables|Default|GetStartLocation)) _alpha) false false))
    (:Finished
      (CallFunction|MovefromStartLocation))))

(event EventBeginPlay
  (Transformation|SetWorldLocation (Variables|Default|GetCloud) (Transformation|GetWorldLocation (Variables|Default|GetStartLocation)) false false)
  (CallFunction|MovefromStartLocation))

(fn ConstructionScript)

(fn RandomizeScale
  (bind _returnvalue (Math|Random|RandomFloatinRange 0.3 1.3))
  (bind _cloud (Variables|Default|GetCloud))
  (bind _returnvalue_2 (Transformation|GetWorldTransform _cloud))
  (Transformation|SetWorldTransform (Variables|Default|GetCloud) (Math|Transform|MakeTransform (.location _returnvalue_2) (.rotation _returnvalue_2) (Math|Vector|MakeVector _returnvalue _returnvalue _returnvalue)) false false))