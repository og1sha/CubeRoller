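; Enemy spawner that drops EnemyBox hazards from above the player pawn on a looping SpawnSpeed timer.
; Each tick picks either a scattered burst, with one box near the player's Y and two or three at random Y, or SpawnWave2.
; SpawnWave2 fills distinct random lanes from nine fixed Y positions, using GetRandomLanes to reroll duplicates.
; SpawnWave, an alternative capped coin-flip lane pattern, is never called.
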(event Custom|SpawnHazard
  (if (Math|Random|RandomBoolwithWeight 0.5)
    (CallFunction|SpawnEnemyActor false)
    (CallFunction|SpawnEnemyActor true)
    (CallFunction|SpawnEnemyActor true)
    (if (Math|Random|RandomBoolwithWeight 0.5)
      (CallFunction|SpawnEnemyActor true))
    (else
      (CallFunction|SpawnWave2))))

(event EventBeginPlay
  (Utilities|Time|SetTimerbyEvent (delegate Custom|SpawnHazard) (Variables|Default|GetSpawnSpeed) true)
  (bind _asbase_pawn (Utilities|Casting|CastToBasePawn (Game|Player|GetPlayerPawn 0)))
  (Variables|Default|SetPawnMesh (Variables|/Game/Blueprints/Character/BasePawn.BasePawn_C|GetPawnMesh _asbase_pawn)))

(fn ConstructionScript)

(fn SpawnEnemyActor
  (params (UseRandomLocation :type Boolean))
  (bind _pawnmesh (Variables|Default|GetPawnMesh))
  (bind _returnvalue (Transformation|GetWorldLocation _pawnmesh))
  (bind _returnvalue_2 (+ (.z _returnvalue) 8e+02))
  (if UseRandomLocation
    (Game|SpawnActorfromClass "/Game/Blueprints/Enemy/EnemyBox.EnemyBox_C" (Math|Transform|MakeTransform (Math|Vector|MakeVector (.x _returnvalue) (Math|Random|RandomFloatinRange -1.35e+03 -3.9e+02) _returnvalue_2) "0, 0, 0" "1,1,1") "Undefined" 0 0)
    (else
      (Game|SpawnActorfromClass "/Game/Blueprints/Enemy/EnemyBox.EnemyBox_C" (Math|Transform|MakeTransform (Math|Vector|MakeVector (.x _returnvalue) (Math|Random|RandomFloatinRange (- (.y _returnvalue) 5e+01) (+ (.y _returnvalue) 5e+01)) _returnvalue_2) "0, 0, 0" "1,1,1") "Undefined" 0 0))))

(fn SpawnWave
  (Variables|Default|SetEnemyCount 0)
  (bind _emptyspaceexists (CallFunction|TrytoSpawnSingleEnemy -1.31e+03))
  (bind _emptyspaceexists_2 (CallFunction|TrytoSpawnSingleEnemy -1.2e+03))
  (bind _emptyspaceexists_3 (CallFunction|TrytoSpawnSingleEnemy -1.09e+03))
  (bind _emptyspaceexists_4 (CallFunction|TrytoSpawnSingleEnemy -9.8e+02))
  (bind _emptyspaceexists_5 (CallFunction|TrytoSpawnSingleEnemy -8.7e+02))
  (bind _emptyspaceexists_6 (CallFunction|TrytoSpawnSingleEnemy -7.6e+02))
  (bind _emptyspaceexists_7 (CallFunction|TrytoSpawnSingleEnemy -6.5e+02))
  (bind _emptyspaceexists_8 (CallFunction|TrytoSpawnSingleEnemy -5.4e+02))
  (if (Math|Boolean|ORBoolean _emptyspaceexists_8 _emptyspaceexists_7 _emptyspaceexists_6 _emptyspaceexists_5 _emptyspaceexists_4 _emptyspaceexists_3 _emptyspaceexists_2 _emptyspaceexists)
    (CallFunction|TrytoSpawnSingleEnemy -4.3e+02)))

(fn TrytoSpawnSingleEnemy
  (params (LocationY :type Float%20%28single-precision%29))
  (bind _returnvalue (Math|Random|RandomBoolwithWeight 0.5))
  (bind _pawnmesh (Variables|Default|GetPawnMesh))
  (bind _returnvalue_2 (Transformation|GetWorldLocation _pawnmesh))
  (if (and (< (Variables|Default|GetEnemyCount) 4) _returnvalue)
    (Game|SpawnActorfromClass "/Game/Blueprints/Enemy/EnemyBox.EnemyBox_C" (Math|Transform|MakeTransform (Math|Vector|MakeVector (.x _returnvalue_2) LocationY (+ (.z _returnvalue_2) 8e+02)) "0, 0, 0" "1,1,1") "Undefined" 0 0)
    (Math|Integer|IncrementInt (Variables|Default|GetEnemyCount)
      (:%20%20
        (return (not _returnvalue))))))

(fn SpawnWave2
  (bind _pawnmesh (Variables|Default|GetPawnMesh))
  (bind _returnvalue (Transformation|GetWorldLocation _pawnmesh))
  (bind _lanes (CallFunction|GetRandomLanes))
  (for _array_element _lanes
    (switch int _array_element
      (:1
        (LocalVariables|SetlocationToSpawn -1.31e+03))
      (:2
        (LocalVariables|SetlocationToSpawn -1.2e+03))
      (:3
        (LocalVariables|SetlocationToSpawn -1.09e+03))
      (:4
        (LocalVariables|SetlocationToSpawn -9.8e+02))
      (:5
        (LocalVariables|SetlocationToSpawn -8.7e+02))
      (:6
        (LocalVariables|SetlocationToSpawn -7.6e+02))
      (:7
        (LocalVariables|SetlocationToSpawn -6.5e+02))
      (:8
        (LocalVariables|SetlocationToSpawn -5.4e+02))
      (:9
        (LocalVariables|SetlocationToSpawn -4.3e+02)))
    (Game|SpawnActorfromClass "/Game/Blueprints/Enemy/EnemyBox.EnemyBox_C" (Math|Transform|MakeTransform (Math|Vector|MakeVector (.x _returnvalue) (LocalVariables|GetlocationToSpawn) (+ (.z _returnvalue) 8e+02)) "0, 0, 0" "1,1,1") "Undefined" 0 0)))

(fn GetRandomLanes
  (for _index (range 0 (Variables|Default|GetMaxEnemyCountInWave))
    (LocalVariables|SetrandomValue (Math|Random|RandomIntegerinRange 1 9))
    (while (Utilities|Array|ContainsItem (LocalVariables|GetlocalLanes) (LocalVariables|GetrandomValue))
      (LocalVariables|SetrandomValue (Math|Random|RandomIntegerinRange 1 9)))
    (Utilities|Array|Add (LocalVariables|GetlocalLanes) (LocalVariables|GetrandomValue)))
  (return (LocalVariables|GetlocalLanes)))