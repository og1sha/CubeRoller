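; EnemyBox is an enemy box that explodes on contact and kills any BasePawn that touches it.
; Its construction script gives the mesh a random scale on each axis, so boxes vary in shape and size.
; Any actor overlap spawns an explosion particle slightly offset along world X and destroys the box, then calls Die on the other actor if it is a BasePawn.
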(event Collision|EventActorBeginOverlap
  (params (OtherActor :type Actor%20Object%20Reference))
  (CallFunction|SpawnDestroyParticle)
  (bind _asbase_pawn (Utilities|Casting|CastToBasePawn OtherActor))
  (Default|Die _asbase_pawn))

(fn ConstructionScript
  (bind _returnvalue (Math|Random|RandomFloatinRange 0.3 1.0))
  (Transformation|SetWorldScale3D (Variables|Default|GetEnemyMesh) (Math|Vector|MakeVector _returnvalue _returnvalue _returnvalue)))

(fn SpawnDestroyParticle
  (bind _returnvalue (Transformation|GetActorLocation))
  (Effects|SpawnEmitteratLocation "/Game/Particles/ExplosionParticle.ExplosionParticle" (Math|Vector|MakeVector (+ (.x _returnvalue) 5e+01) (.y _returnvalue) (.z _returnvalue)))
  (Actor|DestroyActor))