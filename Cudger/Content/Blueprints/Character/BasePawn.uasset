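; Base player pawn for a dodging-style game that moves sideways by physics impulses and earns one score point per second alive.
; Keyboard A/D or device tilt with a dead zone feed ApplyImpulse on the mesh along Y.
; Die locks input, fires the game-over dispatcher, stops the score timer, plays particles, saves any new high score, shows the GameOver widget, then pauses after a short delay.
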(event Custom|IncreaseScore
  ;[1 1 1] Counting score
  (Math|Integer|IncrementInt (Variables|Default|GetScore)))

(event Custom|Die
  (if (not (Variables|Default|GetIsDead))
    (Variables|Default|SetIsDead true)
    (Variables|Default|SetInputDisabled true)
    (Default|CallGameOverEventDispatcher)
    (Utilities|Time|ClearandInvalidateTimerbyHandle (Variables|Default|GetScoreHandler))
    (Components|Activation|Activate (Variables|Default|GetDeathParticle) false)
    (CallFunction|LoadSaveHighScore)
    (Viewport|RemoveAllWidgets)
    (bind _returnvalue (UserInterface|CreateWidget "/Game/UI/GameOver.GameOver_C"))
    (UserInterface|Viewport|AddtoViewport _returnvalue 0)
    (Utilities|FlowControl|Delay 0.6)
    (Game|SetGamePaused true)))

(event EventBeginPlay
  ;[1 1 1] Prevent screensaver from turning on
  (Class|KismetSystemLibrary|ControlScreensaver false)
  ;[1 1 1] Counting score
  (bind _returnvalue (Utilities|Time|SetTimerbyEvent (delegate Custom|IncreaseScore) 1.0 true))
  (Variables|Default|SetScoreHandler _returnvalue)
  (Variables|Default|SetInputDisabled false)
  (Variables|Default|SetIsDead false))

(event Input|KeyboardEvents|A
  (params (Key :type Key%20Structure))
  ;[1 1 1] Keyboard input
  (:Pressed
    (if (not (Variables|Default|GetInputDisabled))
      (CallFunction|ApplyImpulse (* (Variables|Default|GetSpeed) -1e+01)))))

(event Input|KeyboardEvents|D
  (params (Key :type Key%20Structure))
  ;[1 1 1] Keyboard input
  (:Pressed
    (if (not (Variables|Default|GetInputDisabled))
      (CallFunction|ApplyImpulse (* (Variables|Default|GetSpeed) 1e+01)))))

(event Input|KeyboardEvents|Tilt
  (params (AxisValue :type Vector :default "0, 0, 0"))
  (bind _speed (Variables|Default|GetSpeed))
  ;[1 1 1] Mobile input
  (if (not (Variables|Default|GetInputDisabled))
    (if (not (Math|Float|InRange(Float) (.y AxisValue) -0.14 0.14))
      (if (> (.y AxisValue) 0.1)
        (CallFunction|ApplyImpulse _speed)
        (else
          (CallFunction|ApplyImpulse (* _speed -1.0)))))))

(fn ConstructionScript)

(fn ApplyImpulse
  (params (Value :type Float%20%28single-precision%29))
  (Physics|AddImpulse (Variables|Default|GetPawnMesh) (Math|Vector|MakeVector 0.0 Value 0.0) "None" false))

(fn LoadSaveHighScore
  (bind _returnvalue (SaveGame|DoesSaveGameExist "HighScore"))
  (if _returnvalue
    (bind _returnvalue_2 (SaveGame|LoadGamefromSlot "HighScore"))
    (bind _output_get (Variables|Default|SetSaveGame _returnvalue_2))
    (bind _asbp_save_game (Utilities|Casting|CastToBP_SaveGame _output_get))
    (if (> (Variables|Default|GetScore) (Variables|/Game/Blueprints/BP_SaveGame.BP_SaveGame_C|GetHighScore _asbp_save_game))
      (Variables|/Game/Blueprints/BP_SaveGame.BP_SaveGame_C|SetHighScore _asbp_save_game (Variables|Default|GetScore))
      (SaveGame|SaveGametoSlot (Variables|Default|GetSaveGame) "HighScore"))
    (else
      (bind _returnvalue_3 (SaveGame|CreateSaveGameObject "/Game/Blueprints/BP_SaveGame.BP_SaveGame_C"))
      (bind _output_get_2 (Variables|Default|SetSaveGame _returnvalue_3))
      (bind _asbp_save_game_2 (Utilities|Casting|CastToBP_SaveGame _output_get_2))
      (Variables|/Game/Blueprints/BP_SaveGame.BP_SaveGame_C|SetHighScore _asbp_save_game_2 (Variables|Default|GetScore))
      (SaveGame|SaveGametoSlot (Variables|Default|GetSaveGame) "HighScore"))))